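; BP_Door is a sliding door actor that moves from its starting position to an EndLocation.
; BeginPlay records the start location, and the OpenDoors event enables Tick to move the door.
; Tick accumulates time and disables itself once RotationTime is reached.
; The lerp alpha divides CurrentTime by itself instead of by RotationTime, so the door snaps to EndLocation rather than sliding gradually.
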(event `self.ReceiveBeginPlay`
  (set `self.StartLocation` (`self.K2_GetActorLocation`)))

(event `/Game/Blueprint/PuzzleInterface.OpenDoors`
  (`self.SetActorTickEnabled` true))

(event `self.ReceiveTick`
  (params (DeltaSeconds :type "Float (single-precision)"))
  (set `self.CurrentTime` (+ DeltaSeconds (`self.CurrentTime`)))
  (`self.K2_SetActorLocation` (`KismetMathLibrary.VLerp` (`self.StartLocation`) (`self.EndLocation`) (/ (`self.CurrentTime`) (`self.CurrentTime`))))
  (if (>= (`self.CurrentTime`) (`self.RotationTime`))
    (`self.SetActorTickEnabled` false)))

(fn `UserConstructionScript`)